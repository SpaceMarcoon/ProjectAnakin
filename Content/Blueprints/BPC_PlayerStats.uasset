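; Player stats component that tracks current and maximum health and stamina.
; Callable functions subtract, raise maximums or restore values, with healing and stamina restores capped at their maximums; events are empty.
; Both decrease functions return whether CurrentHP is depleted, so DecreaseStamina tests health instead of stamina.
; IncreaseMaxHealth sets MaxHP to zero, leaving its addition unused.
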(event EventBeginPlay)

(event EventTick
  (params (DeltaSeconds :type Float%20%28single-precision%29)))

(fn DecreaseHealth
  (params (Damage :type Float%20%28double-precision%29))
  (Variables|Health|SetCurrent%20HP (- (Variables|Health|GetCurrent%20HP) Damage))
  (if (<= (Variables|Health|GetCurrent%20HP) 0.0)
    (return true)
    (else
      (return false))))

(fn IncreaseMaxHealth
  (params (Increase%20HP :type Float%20%28double-precision%29))
  (Variables|Health|SetMax%20HP 0.0))

(fn DecreaseStamina
  (params (Stamina%20Depleted :type Float%20%28double-precision%29))
  (Variables|Stamina|SetCurrent%20Stamina (- (Variables|Stamina|GetCurrent%20Stamina) Stamina%20Depleted))
  (if (<= (Variables|Health|GetCurrent%20HP) 0.0)
    (return true)
    (else
      (return false))))

(fn IncreaseMaxStamina
  (params (B :type Float%20%28double-precision%29))
  (Variables|Stamina|SetMax%20Stamina (+ (Variables|Stamina|GetMax%20Stamina) B)))

(fn HealHP
  (params (Healing :type Float%20%28double-precision%29))
  (Variables|Health|SetCurrent%20HP (+ (Variables|Health|GetCurrent%20HP) Healing))
  (if (> (Variables|Health|GetCurrent%20HP) (Variables|Health|GetMax%20HP))
    (Variables|Health|SetCurrent%20HP (Variables|Health|GetMax%20HP))))

(fn RestoreStamina
  (params (Stamina%20Added :type Float%20%28double-precision%29))
  (Variables|Stamina|SetCurrent%20Stamina (+ (Variables|Stamina|GetCurrent%20Stamina) Stamina%20Added))
  (if (> (Variables|Stamina|GetCurrent%20Stamina) (Variables|Stamina|GetMax%20Stamina))
    (Variables|Stamina|SetCurrent%20Stamina (Variables|Stamina|GetMax%20Stamina))))